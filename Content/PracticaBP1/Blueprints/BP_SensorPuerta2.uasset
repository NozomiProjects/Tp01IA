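; Pressure-plate sensor that opens and closes a referenced BP_Puerta2 door when the third-person character steps on or off it.
; Box overlaps set a pressed flag, then after a half-second delay set the door's open flag and call its open/close function.
; Tick lerps the Cube toward a slightly lowered position while pressed and back to its BeginPlay location when released, scaled by delta time.
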(event `self.ReceiveBeginPlay`
  (bind _output_get (set `self.PrimeraPosicion` (`SceneComponent.K2_GetComponentLocation` (`self.Cube`)))))

(event `self.ReceiveTick`
  (params (DeltaSeconds :type "Float (single-precision)"))
  (bind _cube (`self.Cube`))
  (bind _returnvalue (`SceneComponent.K2_GetComponentLocation` (`self.Cube`)))
  (bind _returnvalue_2 (* (`GameplayStatics.GetWorldDeltaSeconds`) 2.0))
  (if (`self.BotonPresionado2?`)
    (bind _output_get (set `self.NuevaPosicion` (- (stale `self.ReceiveBeginPlay` _output_get) (0.0 0.0 8.0))))
    (`SceneComponent.K2_SetWorldLocation` _cube (`KismetMathLibrary.VLerp` _returnvalue _output_get _returnvalue_2) false false)
    (else
      (`SceneComponent.K2_SetWorldLocation` _cube (`KismetMathLibrary.VLerp` _returnvalue (stale `self.ReceiveBeginPlay` _output_get) _returnvalue_2) false false))))

(event `self.Box.OnComponentBeginOverlap`
  (params (OverlappedComponent :type "PrimitiveComponent Object Reference") (OtherActor :type "Actor Object Reference") (OtherComp :type "PrimitiveComponent Object Reference") (OtherBodyIndex :type Integer) (bFromSweep :type Boolean) (SweepResult :type "HitResult Structure (by ref)"))
  (bind _refbp_puerta2 (`self.RefBP_Puerta2`))
  (cast `/Game/ThirdPerson/Blueprints/BP_ThirdPersonCharacter` OtherActor)
  (set `self.BotonPresionado2?` true)
  (`KismetSystemLibrary.Delay` 0.5)
  (set `/Game/PracticaBP1/Blueprints/BP_ParedMovediza2.AbrirPuerta2` true _refbp_puerta2)
  (`/Game/PracticaBP1/Blueprints/BP_ParedMovediza2.AbrirOCerrarPuerta2` _refbp_puerta2))

(event `self.Box.OnComponentEndOverlap`
  (params (OverlappedComponent :type "PrimitiveComponent Object Reference") (OtherActor :type "Actor Object Reference") (OtherComp :type "PrimitiveComponent Object Reference") (OtherBodyIndex :type Integer))
  (bind _refbp_puerta2 (`self.RefBP_Puerta2`))
  (cast `/Game/ThirdPerson/Blueprints/BP_ThirdPersonCharacter` OtherActor)
  (set `self.BotonPresionado2?` false)
  (`KismetSystemLibrary.Delay` 0.5)
  (set `/Game/PracticaBP1/Blueprints/BP_ParedMovediza2.AbrirPuerta2` false _refbp_puerta2)
  (`/Game/PracticaBP1/Blueprints/BP_ParedMovediza2.AbrirOCerrarPuerta2` _refbp_puerta2))

(fn `UserConstructionScript`)