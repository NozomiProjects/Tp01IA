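; BP_TorretaFire is a turret that turns to track the player character, with no firing logic in this graph.
; Each Tick it line traces on Visibility from its Cube to the player and only rotates when nothing blocks the trace.
; The Cube eases toward the look-at rotation with RInterpTo, with pitch clamped to a narrow range from level to slightly raised.
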(event `self.ReceiveTick`
  (params (DeltaSeconds :type "Float (single-precision)"))
  (bind _returnvalue (`SceneComponent.K2_GetComponentLocation` (`self.Cube`)))
  (bind _returnvalue_2 (`SceneComponent.K2_GetComponentLocation` (`Actor.RootComponent` (`GameplayStatics.GetPlayerCharacter` 0))))
  (bind (_outhit _returnvalue_3) (`KismetSystemLibrary.LineTraceSingle` _returnvalue _returnvalue_2 "TraceTypeQuery1"))
  (if (not _returnvalue_3)
    (`SceneComponent.K2_SetWorldRotation` (`self.Cube`) (`KismetMathLibrary.MakeRotator` (.roll (`KismetMathLibrary.RInterpTo` (`SceneComponent.K2_GetComponentRotation` (`self.Cube`)) (`KismetMathLibrary.FindLookAtRotation` _returnvalue _returnvalue_2) (`GameplayStatics.GetWorldDeltaSeconds`) 3.0)) (`KismetMathLibrary.ClampAngle` (.pitch (`KismetMathLibrary.RInterpTo` (`SceneComponent.K2_GetComponentRotation` (`self.Cube`)) (`KismetMathLibrary.FindLookAtRotation` _returnvalue _returnvalue_2) (`GameplayStatics.GetWorldDeltaSeconds`) 3.0)) 0.0 15.0) (.yaw (`KismetMathLibrary.RInterpTo` (`SceneComponent.K2_GetComponentRotation` (`self.Cube`)) (`KismetMathLibrary.FindLookAtRotation` _returnvalue _returnvalue_2) (`GameplayStatics.GetWorldDeltaSeconds`) 3.0))) false false)))

(event `self.ReceiveBeginPlay`)

(fn `UserConstructionScript`)