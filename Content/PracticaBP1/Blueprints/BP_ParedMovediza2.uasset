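; Sliding wall that works as a door, opened or closed according to the AbrirPuerta2 flag, which this graph only reads.
; Tick eases the cube from its BeginPlay position toward an offset, along Z if its world yaw is nonzero, otherwise along X, and back when closed, lerping by delta time.
; AbrirOCerrarPuerta2 plays or reverses a Timeline that drives the cube's world scale.
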(event `MoverPuerta2`)

(event `self.ReceiveBeginPlay`
  (`|ExecutionSequence`
    (:`then_0`
      (bind _output_get (set `self.PrimeraPosicion` (`SceneComponent.K2_GetComponentLocation` (`self.Cube`)))))))

(event `self.ReceiveTick`
  (params (DeltaSeconds :type "Float (single-precision)"))
  (bind _returnvalue (`GameplayStatics.GetWorldDeltaSeconds`))
  (bind _primeraposicion (`self.PrimeraPosicion`))
  (bind _cube (`self.Cube`))
  (bind _returnvalue_2 (`SceneComponent.K2_GetComponentLocation` (`self.Cube`)))
  (`|ExecutionSequence`
    (:`then_0`
      (if (`self.AbrirPuerta2`)
        (if (!= (.yaw (`SceneComponent.K2_GetComponentRotation` (`self.Cube`))) 0.0)
          (bind _output_get (set `self.NuevaPosicion` (+ _primeraposicion (0.0 0.0 45.0))))
          (`SceneComponent.K2_SetWorldLocation` _cube (`KismetMathLibrary.VLerp` _returnvalue_2 _output_get _returnvalue) false false)
          (else
            (bind _output_get_2 (set `self.NuevaPosicion` (+ _primeraposicion (45.0 0.0 0.0))))
            (`SceneComponent.K2_SetWorldLocation` _cube (`KismetMathLibrary.VLerp` _returnvalue_2 _output_get_2 _returnvalue) false false)))
        (else
          (`SceneComponent.K2_SetWorldLocation` _cube (`KismetMathLibrary.VLerp` _returnvalue_2 (stale `self.ReceiveBeginPlay` _output_get) _returnvalue) false false))))))

(event `AbrirOCerrarPuerta2`
  (if (`self.AbrirPuerta2`)
    (bind (_direction _nuevaescalax) (`Timeline|Timeline` :!label _label)
      (:`Update`
        (`SceneComponent.SetWorldScale3D` (`self.Cube`) _nuevaescalax)))
    (else
      (goto _label :!via `Reverse`))))

(fn `UserConstructionScript`)