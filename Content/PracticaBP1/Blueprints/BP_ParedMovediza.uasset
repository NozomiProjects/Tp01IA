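; BP_ParedMovediza is a moving wall that opens and closes like a door, driven by the AbrirPuerta flag.
; Tick eases the Cube with a delta-time lerp toward an offset from its starting position, choosing axis and direction by whether its yaw is non-zero, and returns it faster when closing.
; AbrirOCerrarPuerta plays or reverses a timeline that rescales the Cube according to the same flag, which this Blueprint only reads.
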(event `self.ReceiveBeginPlay`
  (bind _output_get (set `self.PrimeraPosicion` (`SceneComponent.K2_GetComponentLocation` (`self.Cube`)))))

(event `self.ReceiveTick`
  (params (DeltaSeconds :type "Float (single-precision)"))
  (bind _returnvalue (`GameplayStatics.GetWorldDeltaSeconds`))
  (bind _cube (`self.Cube`))
  (bind _cube_2 (`self.Cube`))
  (bind _returnvalue_2 (`SceneComponent.K2_GetComponentLocation` _cube))
  (bind _returnvalue_3 (* _returnvalue 0.25))
  (if (`self.AbrirPuerta`)
    (if (!= (.yaw (`SceneComponent.K2_GetComponentRotation` _cube)) 0.0)
      (bind _output_get (set `self.NuevaPosicion` (+ (stale `self.ReceiveBeginPlay` _output_get) (0.0 90.0 0.0))))
      (`SceneComponent.K2_SetWorldLocation` _cube_2 (`KismetMathLibrary.VLerp` _returnvalue_2 _output_get _returnvalue_3) false false)
      (else
        (bind _output_get_2 (set `self.NuevaPosicion` (- (stale `self.ReceiveBeginPlay` _output_get) (90.0 0.0 0.0))))
        (`SceneComponent.K2_SetWorldLocation` _cube_2 (`KismetMathLibrary.VLerp` _returnvalue_2 _output_get_2 _returnvalue_3) false false)))
    (else
      (`SceneComponent.K2_SetWorldLocation` _cube_2 (`KismetMathLibrary.VLerp` _returnvalue_2 (stale `self.ReceiveBeginPlay` _output_get) _returnvalue) false false))))

(event `AbrirOCerrarPuerta`
  (if (`self.AbrirPuerta`)
    (bind (_direction _nuevaescalax) (`Timeline|Timeline_AbrirPuerta` :!label _label)
      (:`Update`
        (`SceneComponent.SetWorldScale3D` (`self.Cube`) _nuevaescalax)))
    (else
      (goto _label :!via `Reverse`))))

(fn `UserConstructionScript`)